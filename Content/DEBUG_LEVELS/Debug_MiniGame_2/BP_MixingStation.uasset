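; Mixing station for Minigame 2 that animates two chemicals combining into either a product or an explosion.
; It hands itself to its 3D screen widget and finds the minigame actor on BeginPlay.
; SpawnElements creates both chemicals, and a timeline lerps them to the center.
; They vanish in smoke, then the minigame's Correct flag selects a temporary product or boom particles before delays end and the widget wakes.
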(event `self.ReceiveBeginPlay`
  (bind _aswbp_minigame_2 (cast `/Game/FirstPerson/Blueprints/Widgets/WBP_Minigame-2` (`WidgetComponent.GetUserWidgetObject` (`self.3D_Screen`)))
    (:`then`
      (set `/Game/FirstPerson/Blueprints/Widgets/WBP_Minigame-2.Mixing Station Ref` self _aswbp_minigame_2)
      (bind _returnvalue (`GameplayStatics.GetActorOfClass` "/Game/FirstPerson/AnimationBlueprints/Utilities/BP_Minigame_2.BP_Minigame_2_C"))
      (set `self.Minigame2 Reference` _returnvalue)
      (add `PrimitiveComponent.OnClicked` (`self.3D_Screen`) (`|CreateDelegate` :!event `OnClicked_Event`)))
    (:`CastFailed`
      (`KismetSystemLibrary.PrintString` "Cast to WBP_Minigame_2_failed"))))

(event `Spawn Elements`
  ; Spwan or boom
  (`KismetSystemLibrary.PrintString` "Station received the call")
  (bind _returnvalue (`|SpawnActorFromClass` "/Game/DEBUG_LEVELS/Debug_MiniGame_2/BP_Chemical.BP_Chemical_C" (`SceneComponent.K2_GetComponentToWorld` (`self.Element A`)) "Undefined" "MultiplyWithRoot" null null))
  (set `self.Chemical_A_Ref` _returnvalue)
  (bind _returnvalue_2 (`|SpawnActorFromClass` "/Game/DEBUG_LEVELS/Debug_MiniGame_2/BP_Chemical.BP_Chemical_C" (`SceneComponent.K2_GetComponentToWorld` (`self.Element B`)) "Undefined" "MultiplyWithRoot" null null))
  (set `self.Chemical_B_Ref` _returnvalue_2)
  (`self.Combine Elements`))

(event `Combined or Boom'd`
  (params (`Success?` :type Boolean))
  ; Spwan or boom
  (`self.K2_DestroyActor` (`self.Chemical_A_Ref`))
  (`self.K2_DestroyActor` (`self.Chemical_B_Ref`))
  (`NiagaraFunctionLibrary.SpawnSystemAtLocation` "/Game/DEBUG_LEVELS/Debug_MiniGame_2/Smoke_effec_System.Smoke_effec_System" (`SceneComponent.K2_GetComponentLocation` (`self.Center Point`)))
  (`KismetSystemLibrary.Delay` 3.5)
  (if `Success?`
    (bind _returnvalue (`|SpawnActorFromClass` "/Game/DEBUG_LEVELS/Debug_MiniGame_2/BP_FinalProduct.BP_FinalProduct_C" (`SceneComponent.K2_GetComponentToWorld` (`self.Center Point`)) "Undefined" "MultiplyWithRoot" null null))
    (`KismetSystemLibrary.Delay` 2.0)
    (`self.K2_DestroyActor` _returnvalue)
    (else
      (`KismetSystemLibrary.PrintString` "Boom Effect ")
      (`NiagaraFunctionLibrary.SpawnSystemAtLocation` "/Game/DEBUG_LEVELS/Debug_MiniGame_2/Particals_Effects_System.Particals_Effects_System" (`SceneComponent.K2_GetComponentLocation` (`self.Center Point`)))
      (`KismetSystemLibrary.Delay` 7.5)))
  (bind _aswbp_minigame_2 (cast `/Game/FirstPerson/Blueprints/Widgets/WBP_Minigame-2` (`WidgetComponent.GetUserWidgetObject` (`self.3D_Screen`))))
  (`/Game/FirstPerson/Blueprints/Widgets/WBP_Minigame-2.WakeUpUI` _aswbp_minigame_2)
  (`KismetSystemLibrary.PrintString` "Woke up"))

(event `self.ReceiveTick`
  (params (DeltaSeconds :type "Float (single-precision)"))
  ; For Rotating the Praticals
)

(event `Combine Elements`
  ; Spwan or boom
  (bind (_direction _alpha) (`Timeline|Timeline_0` :!via `PlayFromStart`)
    (:`Update`
      (`self.K2_SetActorLocation` (`self.Chemical_A_Ref`) (`KismetMathLibrary.VLerp` (`SceneComponent.K2_GetComponentLocation` (`self.Element A`)) (`SceneComponent.K2_GetComponentLocation` (`self.Center Point`)) _alpha) false false)
      (`self.K2_SetActorLocation` (`self.Chemical_B_Ref`) (`KismetMathLibrary.VLerp` (`SceneComponent.K2_GetComponentLocation` (`self.Element B`)) (`SceneComponent.K2_GetComponentLocation` (`self.Center Point`)) _alpha) false false))
    (:`Finished`
      (`self.Combined or Boom'd` (`/Game/FirstPerson/AnimationBlueprints/Utilities/BP_Minigame_2.Correct?` (`self.Minigame2 Reference`))))))

(event `OnClicked_Event`
  (params (TouchedComponent :type "PrimitiveComponent Object Reference") (ButtonPressed :type "Key Structure" :default "None"))
  (`KismetSystemLibrary.PrintString` (`KismetSystemLibrary.GetDisplayName` TouchedComponent)))

(fn `UserConstructionScript`)