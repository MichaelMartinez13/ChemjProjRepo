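; Mixing station actor for the chemistry minigame, hosting its 3D screen widget and showing the result of each element combination.
; SpawnElements creates two chemicals that a timeline lerps to the center, then branches on the minigame's Correct flag.
; Success flashes a product and banks points; failure explodes and cracks the glass, launching and disabling the player when shattered.
; ResetLevel restores the glass and spawns a scored product at the teleport spot.
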(event `OnClicked_Event`
  (params (TouchedComponent :type "PrimitiveComponent Object Reference") (ButtonPressed :type "Key Structure" :default "None"))
  (`KismetSystemLibrary.PrintString` (`KismetSystemLibrary.GetDisplayName` TouchedComponent)))

(event `Reset Level`
  ; For reseting the glass, When Pressed Exit
  (`PrimitiveComponent.SetMaterial` (`self.Glass`) 0 (select `int` 0 :`0` "/Game/textures/ImportedMaterials/Building/glass_Mat.glass_Mat" :`1` null :!type "MaterialInterface Object Reference"))
  (`KismetSystemLibrary.PrintString` "Reset Success from mixing station")
  (if (== 0 (`self.PointTotal`))
    (`KismetSystemLibrary.PrintString` "no points no spawns")
    (else
      (bind _returnvalue (`|SpawnActorFromClass` "/Game/DEBUG_LEVELS/Debug_MiniGame_2/Minigame_2_Material/BP_FinalProduct.BP_FinalProduct_C" (`SceneComponent.K2_GetComponentToWorld` (`self.Teleport Spot`)) "Undefined" "MultiplyWithRoot" null null))
      (`/Game/DEBUG_LEVELS/Debug_MiniGame_2/Minigame_2_Material/BP_FinalProduct.Point Counter` _returnvalue)
      (set `self.PointTotal` 0))))

(event `self.ReceiveBeginPlay`
  (bind _aswbp_minigame_2 (cast `/Game/FirstPerson/Blueprints/Widgets/WBP_Minigame-2` (`WidgetComponent.GetUserWidgetObject` (`self.3D_Screen`)))
    (:`then`
      (set `/Game/FirstPerson/Blueprints/Widgets/WBP_Minigame-2.Mixing Station Ref` self _aswbp_minigame_2)
      (bind _returnvalue (`GameplayStatics.GetActorOfClass` "/Game/FirstPerson/AnimationBlueprints/Utilities/BP_Minigame_2.BP_Minigame_2_C"))
      (set `self.Minigame2 Reference` _returnvalue)
      (add `PrimitiveComponent.OnClicked` (`self.3D_Screen`) (`|CreateDelegate` :!event `OnClicked_Event`))
      (bind _returnvalue_2 (`GameplayStatics.GetActorOfClass` "/Game/DEBUG_LEVELS/Debug_MiniGame_2/Minigame_2_Material/BP_FinalProduct.BP_FinalProduct_C"))
      (set `self.FinalProduct` _returnvalue_2))
    (:`CastFailed`
      (`KismetSystemLibrary.PrintString` "Cast to WBP_Minigame_2_failed"))))

(event `Spawn Elements`
  (params (`Symbol A` :type Integer) (`Symbol B` :type Integer) (GlassDamageLevel :type Integer))
  ; Spwan and boom
  (set `self.Glass Damage Level` GlassDamageLevel)
  (bind _returnvalue (`|SpawnActorFromClass` "/Game/DEBUG_LEVELS/Debug_MiniGame_2/Minigame_2_Material/BP_Chemical.BP_Chemical_C" (`SceneComponent.K2_GetComponentToWorld` (`self.Element A`)) "Undefined" "MultiplyWithRoot" null (`KismetStringLibrary.Conv_IntToString` `Symbol A`) null))
  (set `self.Chemical_A_Ref` _returnvalue)
  (bind _returnvalue_2 (`|SpawnActorFromClass` "/Game/DEBUG_LEVELS/Debug_MiniGame_2/Minigame_2_Material/BP_Chemical.BP_Chemical_C" (`SceneComponent.K2_GetComponentToWorld` (`self.Element B`)) "Undefined" "MultiplyWithRoot" null (`KismetStringLibrary.Conv_IntToString` `Symbol B`) null))
  (set `self.Chemical_B_Ref` _returnvalue_2)
  (`self.Combine Elements`)
  (`KismetSystemLibrary.Delay` 1.25)
  (`NiagaraFunctionLibrary.SpawnSystemAtLocation` "/Game/DEBUG_LEVELS/Debug_MiniGame_2/CloudSmoke_Effect_System.CloudSmoke_Effect_System" (`SceneComponent.K2_GetComponentLocation` (`self.Center Point`))))

(event `Glass Breaking`
  ; For Changing the Glass Breaking Material
  (`PrimitiveComponent.SetMaterial` (`self.Glass`) 0 (select `int` (`self.Glass Damage Level`) :`0` null :`1` "/Game/textures/ImportedMaterials/Building/glassslightlybroken_Mat.glassslightlybroken_Mat" :`2` "/Game/textures/ImportedMaterials/Building/glassbroken_Mat.glassbroken_Mat" :`3` "/Game/textures/ImportedMaterials/Building/ShatteredGlass_Mat.ShatteredGlass_Mat" :!type "MaterialInterface Object Reference"))
  (if (== 3 (`self.Glass Damage Level`))
    (`self.PushBack`)
    (`self.DisableInput` (`GameplayStatics.GetPlayerCharacter` 0) (`GameplayStatics.GetPlayerController` 0))))

(event `PushBack`
  ; Launching back the player when dead
  (`Character.LaunchCharacter` (`GameplayStatics.GetPlayerCharacter` 0) (0.0 100000.0 5000.0) false false))

(event `Combined or Boom'd`
  (params (`Success?` :type Boolean))
  ; Spwan and boom
  (`self.K2_DestroyActor` (`self.Chemical_A_Ref`))
  (`self.K2_DestroyActor` (`self.Chemical_B_Ref`))
  (if `Success?`
    (bind _returnvalue (`|SpawnActorFromClass` "/Game/DEBUG_LEVELS/Debug_MiniGame_2/Minigame_2_Material/BP_FinalProduct.BP_FinalProduct_C" (`SceneComponent.K2_GetComponentToWorld` (`self.Center Point`)) "Undefined" "MultiplyWithRoot" null null))
    (set `self.FinalProduct` _returnvalue)
    (set `self.PointTotal` (+ (`self.PointTotal`) 10))
    (`KismetSystemLibrary.Delay` 0.75)
    (`self.K2_DestroyActor` (`self.FinalProduct`))
    (else
      (`KismetSystemLibrary.PrintString` "Boom Effect ")
      (`KismetSystemLibrary.Delay` 1.5)
      (`NiagaraFunctionLibrary.SpawnSystemAtLocation` "/Game/DEBUG_LEVELS/Debug_MiniGame_2/Explosion_System.Explosion_System" (`SceneComponent.K2_GetComponentLocation` (`self.Center Point`)))
      (`GameplayStatics.PlaySound2D` "/Game/Audio/SFX/Window_Breaking_Sound.Window_Breaking_Sound" 1.0 1.0 0.0 null null)
      (`self.Glass Breaking`)
      (`KismetSystemLibrary.Delay` 3.0)))
  (bind _aswbp_minigame_2 (cast `/Game/FirstPerson/Blueprints/Widgets/WBP_Minigame-2` (`WidgetComponent.GetUserWidgetObject` (`self.3D_Screen`))))
  (`/Game/FirstPerson/Blueprints/Widgets/WBP_Minigame-2.WakeUpUI` _aswbp_minigame_2))

(event `Combine Elements`
  ; Spwan and boom
  (bind (_direction _alpha) (`Timeline|Timeline_0` :!via `PlayFromStart`)
    (:`Update`
      (`self.K2_SetActorLocation` (`self.Chemical_A_Ref`) (`KismetMathLibrary.VLerp` (`SceneComponent.K2_GetComponentLocation` (`self.Element A`)) (`SceneComponent.K2_GetComponentLocation` (`self.Center Point`)) _alpha) false false)
      (`self.K2_SetActorLocation` (`self.Chemical_B_Ref`) (`KismetMathLibrary.VLerp` (`SceneComponent.K2_GetComponentLocation` (`self.Element B`)) (`SceneComponent.K2_GetComponentLocation` (`self.Center Point`)) _alpha) false false)
      (if (> _alpha 0.78)
        ;; For making the color and the infor about the chemicals Disable
        (`/Game/DEBUG_LEVELS/Debug_MiniGame_2/Minigame_2_Material/BP_Chemical.Hide UI` (`self.Chemical_B_Ref`))
        (`/Game/DEBUG_LEVELS/Debug_MiniGame_2/Minigame_2_Material/BP_Chemical.Hide UI` (`self.Chemical_A_Ref`))))
    (:`Finished`
      (`self.Combined or Boom'd` (`/Game/FirstPerson/AnimationBlueprints/Utilities/BP_Minigame_2.Correct?` (`self.Minigame2 Reference`))))))

(fn `UserConstructionScript`)