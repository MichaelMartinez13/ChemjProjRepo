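; BP_FinalProduct is a debug-level actor that accumulates the final product's selling point from three minigames.
; On BeginPlay it finds the mixing station, Minigame 3 and Minigame 1 actors with GetActorOfClass and caches them, taking the widget reference from Minigame 1.
; Three custom events each add their minigame's points to a shared SellingPoint total, reading Minigame 1's from its widget and the others from the actors.
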(event `self.ReceiveBeginPlay`
  (bind _returnvalue (`GameplayStatics.GetActorOfClass` "/Game/DEBUG_LEVELS/Debug_MiniGame_2/Minigame_2_Material/BP_MixingStation.BP_MixingStation_C"))
  (set `self.MixingStation Ref` _returnvalue)
  (bind _returnvalue_2 (`GameplayStatics.GetActorOfClass` "/Game/FirstPerson/Blueprints/Minigame3/Minigame3_Blueprints/BP_Minigame_3.BP_Minigame_3_C"))
  (set `self.MG3 Ref` _returnvalue_2)
  (bind _returnvalue_3 (`GameplayStatics.GetActorOfClass` "/Game/DEBUG_LEVELS/Debug_Minigame_1/BP_MG1.BP_MG1_C"))
  (set `self.WBP1 Ref` (`/Game/DEBUG_LEVELS/Debug_Minigame_1/BP_MG1.WBP Ref` _returnvalue_3)))

(event `MG1 Points`
  ; Point System For Minigame 1
  (set `self.SellingPoint` (+ (`self.SellingPoint`) (`/Game/DEBUG_LEVELS/Debug_Minigame_1/WBP_MG1.PointsToAdd` (`self.WBP1 Ref`)))))

(event `Point Counter`
  ; Point System For Minigame 2
  (set `self.SellingPoint` (+ (`self.SellingPoint`) (`/Game/DEBUG_LEVELS/Debug_MiniGame_2/Minigame_2_Material/BP_MixingStation.PointTotal` (`self.MixingStation Ref`)))))

(event `MG3 Points`
  ; Point System For Minigame 3
  (set `self.SellingPoint` (+ (`self.SellingPoint`) (`/Game/FirstPerson/Blueprints/Minigame3/Minigame3_Blueprints/BP_Minigame_3.MG3 Total Points` (`self.MG3 Ref`)))))

(fn `UserConstructionScript`)