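; Chemical actor for a debug minigame that displays itself as a periodic-table element chosen by its ReceiverSymbol.
; On BeginPlay it looks up that symbol's row in the DT_Periodic data table.
; The row fills the symbol, atomic number and mass texts of its WBP_ChemicalLabel widget and sets the element color material on the Chemical component.
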(event `self.ReceiveBeginPlay`
  ; For applying the Element on to the chemicals
  (bind _returnvalue (`|GetDataTableRow` "/Game/PeriodicTable_Data_Table/DT_Periodic.DT_Periodic" (`KismetStringLibrary.Conv_StringToName` (`self.ReceiverSymbol`)))
    (:`then`
      (bind _aswbp_chemical_label (cast `/Game/DEBUG_LEVELS/Debug_MiniGame_2/Minigame_2_Material/WBP_ChemicalLabel` (`WidgetComponent.GetUserWidgetObject` (`self.Widget`))))
      (bind (_elementsymbol _atomicnumber _amu _element _elementcolor) (break `/Game/PeriodicTable_Data_Table/S_Periodic` _returnvalue))
      (`TextBlock.SetText` (`/Game/DEBUG_LEVELS/Debug_MiniGame_2/Minigame_2_Material/WBP_ChemicalLabel.Text_Symbol` _aswbp_chemical_label) (`KismetTextLibrary.Conv_StringToText` _elementsymbol))
      (`TextBlock.SetText` (`/Game/DEBUG_LEVELS/Debug_MiniGame_2/Minigame_2_Material/WBP_ChemicalLabel.Text_AtomicNumber` _aswbp_chemical_label) (`KismetTextLibrary.Conv_IntToText` _atomicnumber))
      (`TextBlock.SetText` (`/Game/DEBUG_LEVELS/Debug_MiniGame_2/Minigame_2_Material/WBP_ChemicalLabel.Text_Mass` _aswbp_chemical_label) (`KismetTextLibrary.Conv_DoubleToText` _amu "HalfToEven"))
      (`PrimitiveComponent.SetMaterial` (`self.Chemical`) 0 _elementcolor))))

(fn `UserConstructionScript`)