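; BP_PhysSwitch is a self-resetting physical button for debug Minigame 3 that calls PhysButton on BP_Minigame_3 when something overlaps its capsule.
; An overlap disables the capsule's collision and plays a timeline that lowers the switch mesh.
; After a short delay the timeline reverses, then re-enables the trigger after another delay once raised.
; Slowdown and ResetButtonSpeed both set the same normal play rate, so press and return speeds match.
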(event `self.ReceiveBeginPlay`
  (bind _returnvalue (`GameplayStatics.GetActorOfClass` "/Game/FirstPerson/Blueprints/Minigame3/Minigame3_Blueprints/BP_Minigame_3.BP_Minigame_3_C"))
  (set `self.Minigame3_Ref` _returnvalue))

(event `Trigger Off`
  (`PrimitiveComponent.SetCollisionEnabled` (`self.Capsule`) "NoCollision"))

(event `Reset Button Speed`
  (`TimelineComponent.SetPlayRate` (`self.Button Press`) 1.0))

(event `Slowdown`
  (`TimelineComponent.SetPlayRate` (`self.Button Press`) 1.0))

(event `Trigger On`
  (`PrimitiveComponent.SetCollisionEnabled` (`self.Capsule`) "QueryAndPhysics"))

(event `self.Capsule.OnComponentBeginOverlap`
  (params (OverlappedComponent :type "PrimitiveComponent Object Reference") (OtherActor :type "Actor Object Reference") (OtherComp :type "PrimitiveComponent Object Reference") (OtherBodyIndex :type Integer) (bFromSweep :type Boolean) (SweepResult :type "HitResult Structure (by ref)"))
  (`/Game/FirstPerson/Blueprints/Minigame3/Minigame3_Blueprints/BP_Minigame_3.Phys Button` (`self.Minigame3_Ref`))
  (`self.Trigger Off`)
  (bind (_direction _alpha_value) (`Timeline|Button Press` :!label _label)
    (:`Update`
      (`SceneComponent.K2_SetRelativeLocation` (`self.Button_Switch`) (`KismetMathLibrary.VLerp` (0.0 0.0 100.0) (0.0 0.0 -35.0) _alpha_value) false false))
    (:`Finished`
      (`KismetSystemLibrary.Delay` 0.5)
      (if (== _alpha_value 0.0)
        (`self.Reset Button Speed`)
        (`self.Trigger On`)
        (else
          (`self.Reset Button`))))))

(event `Reset Button`
  (`self.Slowdown`)
  (goto _label :!via `ReverseFromEnd`))

(fn `UserConstructionScript`)