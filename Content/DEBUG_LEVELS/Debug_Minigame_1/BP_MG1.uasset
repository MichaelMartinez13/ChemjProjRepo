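; BP_MG1 is the actor Blueprint for debug Minigame 1, hosting the WBP_MG1 interface through its WorldWidget component.
; On BeginPlay it casts that component's widget to WBP_MG1, stores it and passes itself back as MG1Ref, linking both ways.
; GetWidgetRef exposes the widget.
; The SpawnArrow event is an empty stub, and the FinalProduct MG1Points call is disconnected, so the actor holds no gameplay logic.
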(event `self.ReceiveBeginPlay`
  (bind _aswbp_mg1 (cast `/Game/DEBUG_LEVELS/Debug_Minigame_1/WBP_MG1` (`WidgetComponent.GetWidget` (`self.World Widget`))))
  (bind _output_get (set `self.WBP Ref` _aswbp_mg1))
  (set `/Game/DEBUG_LEVELS/Debug_Minigame_1/WBP_MG1.MG1 Ref` self _output_get))

(event `Spawn Arrow`)

(fn `GetWidgetRef`
  (returns (`Widget Ref` :type "UserWidget Object Reference"))
  (return (`WidgetComponent.GetWidget` (`self.World Widget`))))

(fn `UserConstructionScript`)