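; BP_Button is a pressable button in a debug minigame level, usable with E while the player overlaps its collision.
; Overlap toggles input, and a timeline dips ButtonBit 10 units on press.
; At the bottom it calls ButtonCallToAction, an empty stub here taking an action type and target, then reverses.
; A gate blocks presses during the return and reopens once the button is back up.
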(event `self.ReceiveBeginPlay`
  (set `self.Home Location` (`SceneComponent.RelativeLocation` (`self.button_bit`))))

(event `Key|E`
  (params (Key :type "Key Structure"))
  (bind (_home_location_x _home_location_y _home_location_z) (`KismetMathLibrary.BreakVector` (`self.Home Location`)))
  (:`Pressed`
    (`/Engine/EditorBlueprintResources/StandardMacros.Gate` false :!label _label
      (:`Exit`
        (bind (_direction _alpha) (`Timeline|Timeline` :!label _label_2)
          (:`Update`
            (`SceneComponent.K2_SetRelativeLocation` (`self.button_bit`) (`KismetMathLibrary.MakeVector` _home_location_x _home_location_y (`KismetMathLibrary.Lerp` _home_location_z (- _home_location_z 10.0) _alpha)) false false))
          (:`Finished`
            (if (`KismetMathLibrary.NearlyEqual_FloatFloat` _alpha 1.0)
              (`self.ButtonPressed`)
              (`self.Reverse Timeline`)
              (else
                (`self.Reset Button`)))))))))

(event `self.collision.OnComponentBeginOverlap`
  (params (OverlappedComponent :type "PrimitiveComponent Object Reference") (OtherActor :type "Actor Object Reference") (OtherComp :type "PrimitiveComponent Object Reference") (OtherBodyIndex :type Integer) (bFromSweep :type Boolean) (SweepResult :type "HitResult Structure (by ref)"))
  (`self.EnableInput` (`GameplayStatics.GetPlayerController` 0)))

(event `Reset Button`
  (goto _label :!via `Open`))

(event `Reverse Timeline`
  (`|ExecutionSequence`
    (:`then_0`
      (goto _label :!via `Close`))
    (:`then_1`
      (goto _label_2 :!via `ReverseFromEnd`))))

(event `self.collision.OnComponentEndOverlap`
  (params (OverlappedComponent :type "PrimitiveComponent Object Reference") (OtherActor :type "Actor Object Reference") (OtherComp :type "PrimitiveComponent Object Reference") (OtherBodyIndex :type Integer))
  (`self.DisableInput` (`GameplayStatics.GetPlayerController` 0)))

(event `ButtonPressed`
  (`self.Button-CallToAction` (`self.ButtonAction`) (`self.Target`)))

(fn `Button-CallToAction`
  (params (`Action Type` :type String) (`Action Target` :type "Actor Object Reference")))

(fn `UserConstructionScript`)