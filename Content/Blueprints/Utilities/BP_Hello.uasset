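; BP_Hello is a trigger volume that gives the player a double jump and a temporary size boost.
; When an actor tagged Player overlaps the Box, it prints a greeting and fetches the character through GetPlayerMessage.
; It raises the jump count and doubles the mesh scale, then restores normal scale after a short Delay.
; The jump change is never reverted, and only the mesh is rescaled.
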(event `self.Box.OnComponentBeginOverlap`
  (params (OverlappedComponent :type "PrimitiveComponent Object Reference") (OtherActor :type "Actor Object Reference") (OtherComp :type "PrimitiveComponent Object Reference") (OtherBodyIndex :type Integer) (bFromSweep :type Boolean) (SweepResult :type "HitResult Structure (by ref)"))
  (if (`self.ActorHasTag` OtherActor "Player")
    (`KismetSystemLibrary.PrintString` "Hello")
    (bind _player_ref (message `/Game/Blueprints/Utilities/BPI_Reacher.Get Player` OtherActor))
    (set `Character.JumpMaxCount` 2 _player_ref)
    (bind _mesh (`Character.Mesh` _player_ref))
    (bind _returnvalue (`KismetMathLibrary.MakeTransform` (.location (`SceneComponent.K2_GetComponentToWorld` _mesh)) (.rotation (`SceneComponent.K2_GetComponentToWorld` _mesh)) (2.0 2.0 2.0)))
    (`SceneComponent.K2_SetWorldTransform` _mesh _returnvalue false false)
    (`KismetSystemLibrary.Delay` 3.0)
    (`SceneComponent.K2_SetWorldTransform` _mesh (`KismetMathLibrary.MakeTransform` (.location _returnvalue) (.rotation _returnvalue)) false false)))

(fn `UserConstructionScript`)