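; Chemical equation balancing minigame that draws up to two random periodic table elements and gives them random atom counts on two sides.
; Side A takes a coefficient per element and side B a single shared one, each multiplied into per-element totals and printed on screen.
; FinalMolCheck sets Correct when both total arrays match.
; Remake clears everything and regenerates; BeginPlay is empty, so BeginGame must be called externally.
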(event `Clear Answers`
  (`KismetArrayLibrary.Array_Clear` (`self.A Mol Count`))
  (`KismetArrayLibrary.Array_Clear` (`self.B Mol Count`)))

(event `Remake`
  (`BlueprintMapLibrary.Map_Clear` (`self.Side A`))
  (`BlueprintMapLibrary.Map_Clear` (`self.Side B`))
  (`KismetArrayLibrary.Array_Clear` (`self.A Mol Count`))
  (`KismetArrayLibrary.Array_Clear` (`self.B Mol Count`))
  (`self.Begin Game`))

(event `Begin Game`
  (`self.Side A Setup`))

(event `self.ReceiveBeginPlay`)

(event `Side A Setup`
  (for _ (range 2)
    (bind _returnvalue (`|GetDataTableRow` "/Game/Data_Table/DT_Periodic.DT_Periodic" (`KismetStringLibrary.Conv_StringToName` (`KismetStringLibrary.Conv_IntToString` (`KismetMathLibrary.RandomIntegerInRange` 1 118))))
      (:`then`
        (`BlueprintMapLibrary.Map_Add` (`self.Side A`) (`.AtomicNumber_86_37447A974C59545FF17F048234F09E8C` (break `/Game/Data_Table/S_Periodic` _returnvalue)) (`KismetMathLibrary.RandomIntegerInRange` 1 2)))))
  (`self.Side B  Setup`))

(event `Side A Check`
  (params (A_Inputs :type "Array of Integer"))
  (bind _side_a (`self.Side A`))
  (bind _keys (`BlueprintMapLibrary.Map_Keys` _side_a))
  (for (_array_element _array_index) _keys
    (bind _returnvalue (* (`|GetArrayItem` A_Inputs _array_index) (`BlueprintMapLibrary.Map_Find` _side_a _array_element)))
    (`KismetSystemLibrary.PrintString` (`KismetStringLibrary.Conv_IntToString` _returnvalue) true true (struct :`R` 0.085961 :`G` 1.0 :`A` 1.0) 5.0)
    (`KismetArrayLibrary.Array_Add` (`self.A Mol Count`) _returnvalue)))

(event `Side B  Setup`
  (bind _keys (`BlueprintMapLibrary.Map_Keys` (`self.Side A`)))
  (for _array_element _keys
    (`BlueprintMapLibrary.Map_Add` (`self.Side B`) _array_element (`KismetMathLibrary.RandomIntegerInRange` 1 3))))

(event `Side B Check`
  (params (B_Input :type Integer))
  (bind _side_b (`self.Side B`))
  (bind _keys (`BlueprintMapLibrary.Map_Keys` _side_b))
  (for _array_element _keys
    (bind _returnvalue (* (`BlueprintMapLibrary.Map_Find` _side_b _array_element) B_Input))
    (`KismetSystemLibrary.PrintString` (`KismetStringLibrary.Conv_IntToString` _returnvalue) true true (struct :`G` 0.66 :`B` 1.0 :`A` 1.0) 5.0)
    (`KismetArrayLibrary.Array_Add` (`self.B Mol Count`) _returnvalue)))

(event `Final Mol Check`
  (if (`KismetArrayLibrary.Array_Identical` (`self.A Mol Count`) (`self.B Mol Count`))
    (set `self.Correct?` true)
    (else
      (set `self.Correct?` false))))

(fn `UserConstructionScript`)