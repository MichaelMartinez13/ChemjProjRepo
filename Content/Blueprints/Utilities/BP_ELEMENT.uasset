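; BP_ELEMENT is an actor that displays one periodic table element, with its symbol, atomic number, atomic mass and name.
; The construction script uses ElementNumber as the DT_Periodic row name to fill the text components.
; Each text update also runs a shared SetMaterial call on the Plane, with no material specified.
; Holding C shows a newly created WBP_ELEMENT widget, removed on release, with no element data passed to it.
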(event `self.ReceiveBeginPlay`)

(event `Key|C`
  (params (Key :type "Key Structure"))
  (:`Pressed`
    (bind _returnvalue (`|CreateWidget` "/Game/FirstPerson/Blueprints/Widgets/WBP_ELEMENT.WBP_ELEMENT_C"))
    (`UserWidget.AddToViewport` _returnvalue 0))
  (:`Released`
    (`Widget.RemoveFromParent` _returnvalue)))

(fn `UserConstructionScript`
  (locals (NewLocalVar :type "MaterialInstanceDynamic Object Reference"))
  (bind _returnvalue (`|GetDataTableRow` "/Game/Data_Table/DT_Periodic.DT_Periodic" (`KismetStringLibrary.Conv_StringToName` (`KismetStringLibrary.Conv_IntToString` (`self.Element Number`))))
    (:`then`
      (`|ExecutionSequence`
        (:`then_0`
          (bind (_elementsymbol _atomicnumber _amu _element) (break `/Game/Data_Table/S_Periodic` _returnvalue))
          (`TextRenderComponent.K2_SetText` (`self.Element Symbol Text`) (`KismetTextLibrary.Conv_StringToText` _elementsymbol)))
        (:`then_1`
          (`TextRenderComponent.K2_SetText` (`self.Atomic Number Text`) (`KismetTextLibrary.Conv_IntToText` _atomicnumber)))
        (:`then_2`
          (`TextRenderComponent.K2_SetText` (`self.Atomic Mass Unit Text`) (`KismetTextLibrary.Conv_DoubleToText` _amu "HalfToEven")))
        (:`then_3`
          (`TextRenderComponent.K2_SetText` (`self.Element Name Text`) (`KismetTextLibrary.Conv_StringToText` _element))))
      (`PrimitiveComponent.SetMaterial` (`self.Plane`) 0 null))))